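; Game mode for a tower-defense level that bootstraps the player and gameplay actors on BeginPlay.
; It messages the game instance, spawns and possesses a ThirdPersonCharacter with game-only input, then spawns a TowerBuildingManager.
; It then sends ChainEventMessage to the character, wave manager, enemy spawner and wave-start collision in a fixed order.
; GetDetails returns a constant enumerator.
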(event `self.ReceiveBeginPlay`
  (bind _returnvalue (`GameplayStatics.GetPlayerController` 0))
  (message `/Game/Blueprints/Interfaces/InitiateLevelInstance.GetDetails` (`GameplayStatics.GetGameInstance`))
  (bind _returnvalue_2 (`|SpawnActorFromClass` "/Game/Blueprints/GameCore/ThirdPersonCharacter.ThirdPersonCharacter_C" (`KismetMathLibrary.MakeTransform` (0.0 0.0 750.0)) "Undefined" "OverrideRootScale" null null))
  (bind _output_get (set `self.PlayerCharacter` _returnvalue_2))
  (`Controller.Possess` _returnvalue _output_get)
  (`WidgetBlueprintLibrary.SetInputMode_GameOnly` _returnvalue)
  (`|SpawnActorFromClass` "/Game/Blueprints/TowerPlacing/Actors/TowerBuildingManager.TowerBuildingManager_C" (`KismetMathLibrary.MakeTransform` (0.0 0.0 750.0)) "Undefined" "OverrideRootScale" null null)
  (message `/Game/Blueprints/Interfaces/InitChain.ChainEvent` (`self.PlayerCharacter`))
  (bind _returnvalue_3 (`GameplayStatics.GetActorOfClass` "/Game/w028589a/Wave_Manager/WaveManager.WaveManager_C"))
  (message `/Game/Blueprints/Interfaces/InitChain.ChainEvent` _returnvalue_3)
  (bind _returnvalue_4 (`GameplayStatics.GetActorOfClass` "/Game/d017162l/BP_Enemy_Spawner.BP_Enemy_Spawner_C"))
  (message `/Game/Blueprints/Interfaces/InitChain.ChainEvent` _returnvalue_4)
  (bind _returnvalue_5 (`GameplayStatics.GetActorOfClass` "/Game/w028589a/Wave_Manager/WaveStartCollision_BP.WaveStartCollision_BP_C"))
  (message `/Game/Blueprints/Interfaces/InitChain.ChainEvent` _returnvalue_5))

(fn `GetDetails`
  (returns (GameDifficulty :type "/Game/Blueprints/DataStructures/Enmus/Difficulties Enum"))
  (return "NewEnumerator0"))

(fn `UserConstructionScript`)