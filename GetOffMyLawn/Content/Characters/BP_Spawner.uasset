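; BP_Spawner spawns waves of random enemy types at its location and supplies enemy path waypoints.
; EnemySend sets the count and starts a looping timer for SpawnEnemy, which spawns WaveManager-owned actors and counts down.
; At zero, the timer handle is cleared before the pause call, so the pause misses the timer.
; BeginPlay sorts BP_EnemyPathNode actors into five ordered path arrays, served by GetPathForEnemy, and caches all spawners.
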(event `/Game/Characters/EnemySend.EnemySend`
  (params (BasicEnemy :type Integer) (EnemyType :type "Array of Actor Class Reference (by ref)") (`EnemySpawn Rate` :type "Float (double-precision)"))
  ;[1 1 1] Enemy count
  (set `self.Enemy Count` BasicEnemy)
  ;[1 1 1] Spawner loop
  (if (`KismetSystemLibrary.K2_IsValidTimerHandle` (stale _returnvalue))
    (`KismetSystemLibrary.K2_ClearAndInvalidateTimerHandle` (`self.SpawnerLoop`)))
  (bind _returnvalue (`KismetSystemLibrary.K2_SetTimerDelegate` (delegate `SpawnEnemy`) `EnemySpawn Rate` true))
  (set `self.SpawnerLoop` _returnvalue))

(event `SpawnEnemy`
  ;[1 1 1] Spawner loop
  ;[1 1 1] Spawner of the enemy
  (`|SpawnActorFromClass` (`|GetArrayItem` (stale `/Game/Characters/EnemySend.EnemySend` EnemyType) (`KismetMathLibrary.RandomIntegerInRange` 0 (- (`KismetArrayLibrary.Array_Length` (stale `/Game/Characters/EnemySend.EnemySend` EnemyType)) 1))) (`KismetMathLibrary.MakeTransform` (`self.K2_GetActorLocation`)) "AlwaysSpawn" "OverrideRootScale" (`self.Wave Manager`) null)
  (bind _output_get (set `self.Enemy Count` (- (`self.Enemy Count`) 1)))
  (if (== _output_get 0)
    (bind _output_get_2 (set `self.SpawnerLoop` (struct)))
    (`KismetSystemLibrary.K2_PauseTimerHandle` _output_get_2)))

(event `self.ReceiveBeginPlay`
  (bind _waypointcounts (`self.WaypointCounts`))
  (bind _waypointcounts_2 (`self.WaypointCounts`))
  ;[1 1 1] Setting Path Nodes
  (`|ExecutionSequence`
    (:`then_0`
      (bind _outactors (`GameplayStatics.GetAllActorsOfClass` "/Game/w028589a/BP_EnemyPathNode.BP_EnemyPathNode_C"))
      ;[1 1 1] Counting the number of Enemy Paths
      (`KismetArrayLibrary.Array_Clear` _waypointcounts)
      (`KismetArrayLibrary.Array_Resize` _waypointcounts 5)
      (for _array_element _outactors
        (bind _path (`/Game/w028589a/BP_EnemyPathNode.Path` _array_element))
        (`KismetArrayLibrary.Array_Set` _waypointcounts_2 _path (+ (`|GetArrayItem` _waypointcounts_2 _path) 1)))
      (for _array_element_2 _outactors
        (switch `int` (`/Game/w028589a/BP_EnemyPathNode.Path` _array_element_2)
          (:`0`
            (bind _pathorder (`/Game/w028589a/BP_EnemyPathNode.PathOrder` _array_element_2))
            (`KismetArrayLibrary.Array_Set` (`self.Path0`) _pathorder _array_element_2 true))
          (:`1`
            (`KismetArrayLibrary.Array_Set` (`self.Path1`) _pathorder _array_element_2 true))
          (:`2`
            (`KismetArrayLibrary.Array_Set` (`self.Path2`) _pathorder _array_element_2 true))
          (:`3`
            (`KismetArrayLibrary.Array_Set` (`self.Path3`) _pathorder _array_element_2 true))
          (:`4`
            (`KismetArrayLibrary.Array_Set` (`self.Path4`) _pathorder _array_element_2 true)))))
    (:`then_1`
      (bind _outactors_2 (`GameplayStatics.GetAllActorsOfClass` "BP_Spawner_C"))
      (set `self.Spawners` _outactors_2))))

(fn `GetPathForEnemy`
  (params (Path :type Integer))
  (returns (Waypoints :type "Array of /Game/w028589a/BP_EnemyPathNode Object Reference"))
  (return (select `int` Path :`0` (`self.Path0`) :`1` (`self.Path1`) :`2` (`self.Path2`) :`3` (`self.Path3`) :`4` (`self.Path4`))))

(fn `UserConstructionScript`)