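; Terrain spline actor that builds deformed meshes along an editable spline in the Construction Script, with no runtime logic.
; It adds one spline mesh component per segment, using local point positions and tangents clamped to the total spline length.
; When HasFloor is set, a second pass adds floor segments along the same path, with FloorLength setting their cross-section X scale.
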(fn `UserConstructionScript`
  (bind _spline (`self.Spline`))
  (bind _spline_2 (`self.Spline`))
  (bind _returnvalue (`KismetMathLibrary.MakeVector2D` (`self.FloorLength`) 1.0))
  (bind _returnvalue_2 (- (`SplineComponent.GetNumberOfSplinePoints` _spline_2) 1))
  (bind _returnvalue_3 (- (`SplineComponent.GetNumberOfSplinePoints` _spline) 1))
  (for _index (range (+ _returnvalue_2 1))
    (if (< _index _returnvalue_2)
      (bind _returnvalue_4 (`AddComponent|NODE_AddSplineMeshComponent-0`))
      (bind _returnvalue_5 (+ _index 1))
      (`SplineMeshComponent.SetStartAndEnd` _returnvalue_4 (`SplineComponent.GetLocationAtSplinePoint` _spline_2 _index "Local") (`KismetMathLibrary.ClampVectorSize` (`SplineComponent.GetTangentAtSplinePoint` _spline_2 _index "Local") 0.0 (`SplineComponent.GetSplineLength` _spline_2)) (`SplineComponent.GetLocationAtSplinePoint` _spline_2 _returnvalue_5 "Local") (`KismetMathLibrary.ClampVectorSize` (`SplineComponent.GetTangentAtSplinePoint` _spline_2 _returnvalue_5 "Local") 0.0 (`SplineComponent.GetSplineLength` _spline_2)) true)))
  (if (`self.HasFloor?`)
    (for _index_2 (range (+ _returnvalue_3 1))
      (if (< _index_2 _returnvalue_3)
        (bind _returnvalue_6 (`AddComponent|NODE_AddSplineMeshComponent-1`))
        (bind _returnvalue_7 (+ _index_2 1))
        (`SplineMeshComponent.SetStartAndEnd` _returnvalue_6 (`SplineComponent.GetLocationAtSplinePoint` _spline _index_2 "Local") (`KismetMathLibrary.ClampVectorSize` (`SplineComponent.GetTangentAtSplinePoint` _spline _index_2 "Local") 0.0 (`SplineComponent.GetSplineLength` _spline)) (`SplineComponent.GetLocationAtSplinePoint` _spline _returnvalue_7 "Local") (`KismetMathLibrary.ClampVectorSize` (`SplineComponent.GetTangentAtSplinePoint` _spline _returnvalue_7 "Local") 0.0 (`SplineComponent.GetSplineLength` _spline)) true)
        (`SplineMeshComponent.SetStartScale` _returnvalue_6 _returnvalue true)
        (`SplineMeshComponent.SetEndScale` _returnvalue_6 _returnvalue true)))))