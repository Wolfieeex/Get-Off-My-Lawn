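; Minimap manager actor that creates the minimap widget and converts world positions of the player and enemies into dot coordinates on it.
; On ChainEvent it derives world bounds from TopRight and BottomLeft marker actors and map bounds from the widget's image canvas slot.
; Position functions express an actor's location as a percentage of the world bounds, then scale it to widget coordinates.
; GetEnemyPos and GetPlayerDotPos are unfinished stubs.
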(event `/Game/Blueprints/Interfaces/InitChain.ChainEvent`
  (bind _returnvalue (- (`self.MaxX`) (`self.MinX`)))
  (bind _returnvalue_2 (- (`self.MaxY`) (`self.MinY`)))
  (bind _returnvalue_3 (`WidgetLayoutLibrary.SlotAsCanvasSlot` (`/Game/W012557k/MiniMap/MiniMapBP.Image_13` (`self.WidgetReference`))))
  (bind (_returnvalue_x _returnvalue_y) (`KismetMathLibrary.BreakVector2D` (`CanvasPanelSlot.GetPosition` _returnvalue_3)))
  (bind (_returnvalue_x_2 _returnvalue_y_2) (`KismetMathLibrary.BreakVector2D` (`CanvasPanelSlot.GetSize` _returnvalue_3)))
  (bind _asthird_person_character (cast `/Game/Blueprints/GameCore/ThirdPersonCharacter` (`/Game/Blueprints/GameCore/LevelGameMode.PlayerCharacter` (cast `/Game/Blueprints/GameCore/LevelGameMode` (`GameplayStatics.GetGameMode`) :!pure true))))
  (set `self.PlayerRef` _asthird_person_character)
  (bind _returnvalue_4 (`|CreateWidget` "/Game/W012557k/MiniMap/MiniMapBP.MiniMapBP_C" (`GameplayStatics.GetPlayerController` 0)))
  (bind _output_get (set `self.WidgetReference` _returnvalue_4))
  (`UserWidget.AddToViewport` _output_get 0)
  (bind _returnvalue_5 (`GameplayStatics.GetActorOfClass` "/Game/W012557k/MiniMap/Map_Positions/TopRight.TopRight_C"))
  (bind _output_get_2 (set `self.BottomRightRef` _returnvalue_5))
  (bind (_returnvalue_x_3 _returnvalue_y_3) (`KismetMathLibrary.BreakVector` (`self.K2_GetActorLocation` _output_get_2)))
  (set `self.MaxX` _returnvalue_x_3)
  (set `self.MinY` _returnvalue_y_3)
  (bind _returnvalue_6 (`GameplayStatics.GetActorOfClass` "/Game/W012557k/MiniMap/Map_Positions/BottomLeft.BottomLeft_C"))
  (bind _output_get_3 (set `self.TopLeftRef` _returnvalue_6))
  (bind (_returnvalue_x_4 _returnvalue_y_4) (`KismetMathLibrary.BreakVector` (`self.K2_GetActorLocation` _output_get_3)))
  (set `self.MinX` _returnvalue_x_4)
  (set `self.MaxY` _returnvalue_y_4)
  (set `self.FloatStruct` (make `/Game/W012557k/MiniMap/ActualMapPositionStructs/XYMinMax` (`self.MinX`) (`self.MaxY`) (`self.MaxX`) (`self.MinY`) _returnvalue (/ _returnvalue 100.0) _returnvalue_2 (/ _returnvalue_2 100.0)))
  (bind _output_get_4 (set `self.MapDimensions` (make `/Game/W012557k/MiniMap/MapDimensions` (+ _returnvalue_x _returnvalue_x_2) _returnvalue_x (+ _returnvalue_y _returnvalue_y_2) _returnvalue_y)))
  (set `self.MapPercentages` (make `/Game/W012557k/MiniMap/MapPercentages` (/ (- (- (break `/Game/W012557k/MiniMap/MapDimensions` _output_get_4) 24.0) (`.MinX_12_82174BB1428FF18D9E0E27AE097A8032` (break `/Game/W012557k/MiniMap/MapDimensions` _output_get_4))) 100.0) (/ (- (- (`.MaxY_13_9F2798EE4F015352782A7EBB5B2821DF` (break `/Game/W012557k/MiniMap/MapDimensions` _output_get_4)) 24.0) (`.MinY_14_E2AB6AB746442A930432F2A002E3D641` (break `/Game/W012557k/MiniMap/MapDimensions` _output_get_4))) 100.0))))

(fn `CallInitPlayerDot`
  (`/Game/W012557k/MiniMap/MiniMapBP.InitEnemyDot` (`self.WidgetReference`) null 0))

(fn `GetEnemyPos`)

(fn `GetPlayerDotPos`
  (returns (PlayerX :type "Float (double-precision)") (PlayerY :type "Float (double-precision)"))
  (return 0.0 0.0))

(fn `Set/ Update Player Dot Pos`
  (returns (XPercentage :type "Float (double-precision)") (YPercentage :type "Float (double-precision)") (XCoordinate :type "Float (double-precision)") (YCoordinate :type "Float (double-precision)"))
  (bind (_mapdimensions_maxx _mapdimensions_minx _mapdimensions_maxy _mapdimensions_miny) (break `/Game/W012557k/MiniMap/MapDimensions` (`self.MapDimensions`)))
  (bind (_mappercentages_map1percentxvalue _mappercentages_map1percentyvalue) (break `/Game/W012557k/MiniMap/MapPercentages` (`self.MapPercentages`)))
  (bind (_floatstruct_xmin _floatstruct_ymax _floatstruct_xmax _floatstruct_ymin _floatstruct_xrelativetotal _floatstruct_amountofxfor1percent _floatstruct_yrelativetotal _floatstruct_amountofyfor1percent) (break `/Game/W012557k/MiniMap/ActualMapPositionStructs/XYMinMax` (`self.FloatStruct`)))
  (bind (_returnvalue_x _returnvalue_y) (`KismetMathLibrary.BreakVector` (`self.K2_GetActorLocation` (`self.PlayerRef`))))
  (bind _returnvalue (- _returnvalue_y (`self.MaxY`)))
  (bind _returnvalue_2 (- _returnvalue_x (`self.MinX`)))
  (bind _output_get (set `self.MiniMapRelativePercentages` (make `/Game/W012557k/MiniMap/MiniMapStructs/MiniMapRelativePercentages` _returnvalue_2 (/ _returnvalue_2 _floatstruct_amountofxfor1percent) _returnvalue (/ _returnvalue _floatstruct_amountofyfor1percent))))
  (return (`.XRelativePercentage_7_C30086CA417B397FE88D508B9354F9DE` (break `/Game/W012557k/MiniMap/MiniMapStructs/MiniMapRelativePercentages` _output_get)) (`.YRelativePercentage_10_3FE1F4C041BAD0B053B66D92C4599DA6` (break `/Game/W012557k/MiniMap/MiniMapStructs/MiniMapRelativePercentages` _output_get)) (+ (* (`.XRelativePercentage_7_C30086CA417B397FE88D508B9354F9DE` (break `/Game/W012557k/MiniMap/MiniMapStructs/MiniMapRelativePercentages` _output_get)) _mappercentages_map1percentxvalue) _mapdimensions_minx) (- _mapdimensions_miny (* _mappercentages_map1percentyvalue (`.YRelativePercentage_10_3FE1F4C041BAD0B053B66D92C4599DA6` (break `/Game/W012557k/MiniMap/MiniMapStructs/MiniMapRelativePercentages` _output_get))))))

(fn `SetEnemyPos+Dot`
  (params (EnemyID :type Integer) (EnemyPosition :type "Transform Structure") (`actor ref` :type "Actor Object Reference"))
  (returns (XPercentage :type "Float (double-precision)") (YPercentage :type "Float (double-precision)") (XCoordinate :type "Float (double-precision)") (YCoordinate :type "Float (double-precision)") (EnemyIDThing :type Integer))
  (bind (_returnvalue_x _returnvalue_y) (`KismetMathLibrary.BreakVector` (`self.K2_GetActorLocation` `actor ref`)))
  (bind (_mapdimensions_maxx _mapdimensions_minx _mapdimensions_maxy _mapdimensions_miny) (break `/Game/W012557k/MiniMap/MapDimensions` (`self.MapDimensions`)))
  (bind (_mappercentages_map1percentxvalue _mappercentages_map1percentyvalue) (break `/Game/W012557k/MiniMap/MapPercentages` (`self.MapPercentages`)))
  (bind (_floatstruct_xmin _floatstruct_ymax _floatstruct_xmax _floatstruct_ymin _floatstruct_xrelativetotal _floatstruct_amountofxfor1percent _floatstruct_yrelativetotal _floatstruct_amountofyfor1percent) (break `/Game/W012557k/MiniMap/ActualMapPositionStructs/XYMinMax` (`self.FloatStruct`)))
  (bind _returnvalue (- _returnvalue_y (`self.MaxY`)))
  (bind _returnvalue_2 (- _returnvalue_x (`self.MinX`)))
  (bind _output_get (set `self.MiniMapRelativePercentages` (make `/Game/W012557k/MiniMap/MiniMapStructs/MiniMapRelativePercentages` _returnvalue_2 (/ _returnvalue_2 _floatstruct_amountofxfor1percent) _returnvalue (/ _returnvalue _floatstruct_amountofyfor1percent))))
  (return (`.XRelativePercentage_7_C30086CA417B397FE88D508B9354F9DE` (break `/Game/W012557k/MiniMap/MiniMapStructs/MiniMapRelativePercentages` _output_get)) (`.YRelativePercentage_10_3FE1F4C041BAD0B053B66D92C4599DA6` (break `/Game/W012557k/MiniMap/MiniMapStructs/MiniMapRelativePercentages` _output_get)) (+ (* (`.XRelativePercentage_7_C30086CA417B397FE88D508B9354F9DE` (break `/Game/W012557k/MiniMap/MiniMapStructs/MiniMapRelativePercentages` _output_get)) _mappercentages_map1percentxvalue) _mapdimensions_minx) (- _mapdimensions_miny (* _mappercentages_map1percentyvalue (`.YRelativePercentage_10_3FE1F4C041BAD0B053B66D92C4599DA6` (break `/Game/W012557k/MiniMap/MiniMapStructs/MiniMapRelativePercentages` _output_get)))) EnemyID))

(fn `UserConstructionScript`)