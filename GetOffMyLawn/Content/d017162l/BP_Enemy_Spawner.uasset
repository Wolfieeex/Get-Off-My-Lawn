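; Enemy spawner actor that spawns one MasterEnemy at its own location each time the WaveManager signals a wave start.
; On BeginPlay it finds the WaveManager and binds to its wave start event.
; Each spawned enemy's death decrements the manager's EnemySpawnMax, and at zero or below it triggers the intermission event and resets the count to zero.
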(event `self.ReceiveBeginPlay`
  (bind _returnvalue (`GameplayStatics.GetActorOfClass` "/Game/w028589a/Wave_Manager/WaveManager.WaveManager_C"))
  (bind _output_get (set `self.Wave Manager reference` _returnvalue))
  (add `/Game/w028589a/Wave_Manager/WaveManager.WaveStart` _output_get (delegate `SpawnEnemies`)))

(event `SpawnEnemies`
  (params (WaveManager :type "/Game/w028589a/Wave_Manager/WaveManager Object Reference") (CurrentWave :type Integer) (`FinalWave?` :type Boolean))
  ;[1 1 1] Spawn Enemies
  (bind _returnvalue (`|SpawnActorFromClass` "/Game/w028589a/MasterEnemy.MasterEnemy_C" (`KismetMathLibrary.MakeTransform` (`self.K2_GetActorLocation`)) "Undefined" "OverrideRootScale" null null))
  (add `/Game/w028589a/MasterEnemy.Event Enemy Death` _returnvalue (delegate `EnemyDeathCount`)))

(event `EnemyDeathCount`
  ;[1 1 1] Spawn Enemies
  (bind _result (`/Engine/EditorBlueprintResources/StandardMacros.DecrementInt` (`/Game/w028589a/Wave_Manager/WaveManager.EnemySpawnMax` (`self.Wave Manager reference`)))
    (:`  `
      (if (<= _result 0)
        (`self.EventStartIntermission`)
        (set `self.Enemy Spawn Max` 0)))))

(fn `UserConstructionScript`)