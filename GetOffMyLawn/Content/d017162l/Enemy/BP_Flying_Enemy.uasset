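; Flying enemy Blueprint that fires projectiles and overrides its parent's health and seed-count functions.
; FireProjectile line-traces from the actor toward its world location scaled by 200, then spawns BP_Flying_Projectile at the hit location with zero rotation.
; ModifyHealth adds or subtracts within zero and MaxHealth in the CharacterStats struct.
; GetHealth overwrites Health with a fixed value before returning it, and the debug health display is unconnected.
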(event `self.ReceiveBeginPlay`
  (`parent.ReceiveBeginPlay`))

(event `self.FireProjectile`
  (bind _returnvalue (`self.K2_GetActorLocation`))
  (bind _outhit (`KismetSystemLibrary.LineTraceSingle` _returnvalue (* _returnvalue 200.0) "TraceTypeQuery1" false (`|MakeArray` self :!type "Actor Object Reference") "ForDuration"))
  (`|SpawnActorFromClass` "/Game/d017162l/Enemy/BP_Flying_Projectile.BP_Flying_Projectile_C" (`KismetMathLibrary.MakeTransform` (`.Location` (`GameplayStatics.BreakHitResult` _outhit))) "Undefined" "OverrideRootScale" null null))

(fn `GetHealth`
  (returns (Health :type "Float (double-precision)"))
  (bind _structout (setmembers `/Game/Characters/BS_CharacterStats` :`StructRef` (`self.CharacterStats`) :`Health` 50.0))
  (return (`.Health_9_0A2B731541A6848E04980BB2CB466D3B` (break `/Game/Characters/BS_CharacterStats` _structout))))

(fn `GetSeedCount`
  (returns (SeedCount :type Integer))
  (return (`.SeedCount_10_8B1B175242E26C8AD0EA33A9A109921F` (break `/Game/Characters/BS_CharacterStats` (`self.CharacterStats`)))))

(fn `Modify Health`
  (params (Amount :type "Float (double-precision)") (`Positive?` :type Boolean))
  (locals (L_HealthTemp :type "Float (double-precision)"))
  (set `local.L_HealthTemp` (`.Health_9_0A2B731541A6848E04980BB2CB466D3B` (break `/Game/Characters/BS_CharacterStats` (`self.CharacterStats`))))
  (if (`local.Positive?`)
    (set `local.L_HealthTemp` (+ (`local.L_HealthTemp`) (`local.Amount`)))
    (else
      (set `local.L_HealthTemp` (- (`local.L_HealthTemp`) (`local.Amount`)))))
  (bind _output_get (set `local.L_HealthTemp` (`KismetMathLibrary.FClamp` (`local.L_HealthTemp`) 0.0 (`.MaxHealth_8_0DE6012641829A8ED58B468B27926C98` (break `/Game/Characters/BS_CharacterStats` (`self.CharacterStats`))))))
  (setmembers `/Game/Characters/BS_CharacterStats` :`StructRef` (`self.CharacterStats`) :`Health` _output_get))

(fn `ModifySeedCount`
  (params (Amount :type Integer) (`Positive?` :type Boolean))
  (`parent.ModifySeedCount` Amount `Positive?`))

(fn `UserConstructionScript`
  (`parent.UserConstructionScript`))