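; Flying enemy that fires projectiles while its trigger is overlapped and can drop seeds.
; BeginPlay loads health and DPS from the enemy DataTable; ModifyHealth clamps changes but resets max health to 100.
; UniqueMech overlap starts a looping timer spawning projectiles at FirePoint; end overlap nulls the handle before clearing, so firing never stops.
; DropSeeds traces downward to place a five-seed pickup, and Tick draws debug health.
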(event `self.ReceiveBeginPlay`
  ;[1 1 1] Health
  (`parent.ReceiveBeginPlay`)
  (bind _returnvalue (`|GetDataTableRow` "/Game/W012557k/EnemyDataTable.EnemyDataTable" "Flying")
    (:`then`
      (set `self.NewEnemyStats` (make `/Game/d017162l/Sructs/ST_Master_Enemy` (break `/Game/W012557k/EnemyDataStruct` _returnvalue) (break `/Game/W012557k/EnemyDataStruct` _returnvalue)))
      (set `self.DamagePerSecond` (`.DPS_5_4605C703464A7BBC0F5AB790BF08079B` (break `/Game/W012557k/EnemyDataStruct` _returnvalue))))))

(event `self.ReceiveTick`
  (params (DeltaSeconds :type "Float (single-precision)"))
  (`parent.ReceiveTick` DeltaSeconds)
  (`KismetSystemLibrary.DrawDebugString` (0.0 0.0 100.0) (`KismetStringLibrary.Concat_StrStr` "FlyingEnemy =" (`KismetStringLibrary.Conv_DoubleToString` (`self.GetHealth`))) self))

(event `self.UniqueMech.OnComponentBeginOverlap`
  (params (OverlappedComponent :type "PrimitiveComponent Object Reference") (OtherActor :type "Actor Object Reference") (OtherComp :type "PrimitiveComponent Object Reference") (OtherBodyIndex :type Integer) (bFromSweep :type Boolean) (SweepResult :type "HitResult Structure (by ref)"))
  ;[0 0.1796 1 1 50] Enemy searchging and targetting
  (`KismetSystemLibrary.PrintString` "Fire projectile ")
  (set `self.PlayerInRange` true)
  (set `self.End overlap timer` (struct))
  (if (`self.PlayerInRange`)
    (bind _returnvalue (`KismetSystemLibrary.K2_SetTimerDelegate` (delegate `SpawnProjectile`) 1.0 true))
    (set `self.End overlap timer` _returnvalue)))

(event `self.UniqueMech.OnComponentEndOverlap`
  (params (OverlappedComponent :type "PrimitiveComponent Object Reference") (OtherActor :type "Actor Object Reference") (OtherComp :type "PrimitiveComponent Object Reference") (OtherBodyIndex :type Integer))
  ;[0 0.1796 1 1 50] Enemy searchging and targetting
  (set `self.End overlap timer` (struct))
  (set `self.PlayerInRange` false)
  (`KismetSystemLibrary.K2_ClearAndInvalidateTimerHandle` (`self.End overlap timer`)))

(event `SpawnProjectile`
  (bind (_returnvalue_location _returnvalue_rotation) (`KismetMathLibrary.BreakTransform` (`SceneComponent.K2_GetComponentToWorld` (`self.FirePoint`))))
  ;[0.4103 0.4659 1 1 57] Add projectile
  (`|SpawnActorFromClass` "/Game/d017162l/Enemy/BP_Flying_Projectile.BP_Flying_Projectile_C" (`KismetMathLibrary.MakeTransform` _returnvalue_location _returnvalue_rotation) "Undefined" "OverrideRootScale" null null))

(event `StartShot`
  ;[0 0.1796 1 1 50] Enemy searchging and targetting
)

(event `self.Drop_Seeds `
  (bind _returnvalue (`self.K2_GetActorLocation`))
  ;[0 0 0 1 81] Drop Seed function
  (bind _outhit (`KismetSystemLibrary.LineTraceSingle` _returnvalue (- _returnvalue (0.0 0.0 200.0)) "TraceTypeQuery1" false (`|MakeArray` (`GameplayStatics.GetPlayerCharacter` 0) :!type "Actor Object Reference") "ForOneFrame"))
  (`KismetSystemLibrary.PrintString` "Ground floor detected")
  (bind _returnvalue_2 (`|SpawnActorFromClass` "/Game/w028589a/Seed_Currency/BP_Seed.BP_Seed_C" (`KismetMathLibrary.MakeTransform` (+ (`.Location` (`GameplayStatics.BreakHitResult` _outhit)) (0.0 0.0 50.0))) "Undefined" "OverrideRootScale" null null))
  (set `/Game/w028589a/Seed_Currency/BP_Seed.SeedAmount` 5 _returnvalue_2))

(fn `FireFliyngEnProjectlile`)

(fn `GetHealth`
  (returns (Health :type "Float (double-precision)"))
  (return (`.CurrentHealth_2_5EEBD56E4CBFB0F5442219AF06FBEE13` (break `/Game/d017162l/Sructs/ST_Master_Enemy` (`self.NewEnemyStats`)))))

(fn `GetSeedCount`
  (returns (SeedCount :type Integer))
  (return (`.SeedCount_10_8B1B175242E26C8AD0EA33A9A109921F` (break `/Game/Characters/BS_CharacterStats` (`self.CharacterStats`)))))

(fn `Modify Health`
  (params (Amount :type "Float (double-precision)") (`Positive?` :type Boolean))
  (locals (L_HealthTemp :type "Float (double-precision)"))
  (set `local.L_HealthTemp` (`.CurrentHealth_2_5EEBD56E4CBFB0F5442219AF06FBEE13` (break `/Game/d017162l/Sructs/ST_Master_Enemy` (`self.NewEnemyStats`))))
  (if (`local.Positive?`)
    (set `local.L_HealthTemp` (+ (`local.L_HealthTemp`) (`local.Amount`)))
    (else
      (set `local.L_HealthTemp` (- (`local.L_HealthTemp`) (`local.Amount`)))))
  (bind _output_get (set `local.L_HealthTemp` (`KismetMathLibrary.FClamp` (`local.L_HealthTemp`) 0.0 (`.MaxHealth_4_763AE4A547EB023D3CB181848FF59F59` (break `/Game/d017162l/Sructs/ST_Master_Enemy` (`self.NewEnemyStats`))))))
  (setmembers `/Game/d017162l/Sructs/ST_Master_Enemy` :`StructRef` (`self.NewEnemyStats`) :`CurrentHealth` _output_get :`MaxHealth` 100.0))

(fn `ModifySeedCount`
  (params (Amount :type Integer) (`Positive?` :type Boolean))
  (`parent.ModifySeedCount` Amount `Positive?`))

(fn `UserConstructionScript`
  (`parent.UserConstructionScript`))