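; Test actor for a mushroom pot with a VAT (vertex animation texture) mesh that glows, then scales a mushroom.
; BeginPlay creates a dynamic instance of the VAT material and sets a flag that lets Tick call Play on the Glow timeline.
; Glow drives the emissive parameter; on finish, it swaps the pot to the MushroomUnwrap material and starts a second timeline driving the Mushroom's uniform scale.
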(event `self.ReceiveBeginPlay`
  (bind _returnvalue (`PrimitiveComponent.CreateDynamicMaterialInstance` (`self.MushroomPotVAT_mesh`) 0 "/Game/t017849k/SkeletalMeshes/Flytrap/VATMI_MushroomPotMat.VATMI_MushroomPotMat" "VATMI"))
  (set `self.Instance` _returnvalue)
  (set `self.MaterialSet` true))

(event `self.ReceiveTick`
  (params (DeltaSeconds :type "Float (single-precision)"))
  (if (`self.MaterialSet`)
    (bind (_direction _alpha) (`Timeline|Glow` :`NewTime` 0.0)
      (:`Update`
        (`MeshComponent.SetScalarParameterValueOnMaterials` (`self.MushroomPotVAT_mesh`) "EmissiveGlow" _alpha))
      (:`Finished`
        (`PrimitiveComponent.SetMaterial` (`self.MushroomPotVAT_mesh`) 0 "/Game/t017849k/SkeletalMeshes/Mushroom/MushroomUnwrap.MushroomUnwrap")
        (bind (_direction_2 _alpha_2) (`Timeline|Timeline_0`)
          (:`Update`
            (`SceneComponent.SetRelativeScale3D` (`self.Mushroom`) (`KismetMathLibrary.Conv_DoubleToVector` _alpha_2))))))))

(fn `UserConstructionScript`)