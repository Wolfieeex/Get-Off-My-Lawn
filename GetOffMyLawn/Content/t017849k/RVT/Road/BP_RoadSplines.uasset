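; BP_RoadSplines is a road Blueprint that builds spline meshes along its SplineRoad spline in the construction script.
; Each pair of neighboring points gets an X-forward segment matching their local locations and tangents, with start and end cross-section scale taken from each point's Y and Z scale.
; The first and last segments are tagged with opposite-signed custom primitive data, distinguishing the road's ends.
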(fn `UserConstructionScript`
  (bind _spline_road (`self.Spline_Road`))
  (for _index (range (+ (- (`SplineComponent.GetNumberOfSplinePoints` (`self.Spline_Road`)) 2) 1))
    (bind _returnvalue (`AddComponent|NODE_AddSplineMeshComponent-0`))
    (`SplineMeshComponent.SetForwardAxis` _returnvalue "X" true)
    (bind _returnvalue_2 (+ _index 1))
    (`SplineMeshComponent.SetStartAndEnd` _returnvalue (`SplineComponent.GetLocationAtSplinePoint` _spline_road _index "Local") (`SplineComponent.GetTangentAtSplinePoint` _spline_road _index "Local") (`SplineComponent.GetLocationAtSplinePoint` _spline_road _returnvalue_2 "Local") (`SplineComponent.GetTangentAtSplinePoint` _spline_road _returnvalue_2 "Local") true)
    (bind (_returnvalue_x _returnvalue_y _returnvalue_z) (`KismetMathLibrary.BreakVector` (`SplineComponent.GetScaleAtSplinePoint` _spline_road _index)))
    (`SplineMeshComponent.SetStartScale` _returnvalue (`KismetMathLibrary.MakeVector2D` _returnvalue_y _returnvalue_z) true)
    (bind (_returnvalue_x_2 _returnvalue_y_2 _returnvalue_z_2) (`KismetMathLibrary.BreakVector` (`SplineComponent.GetScaleAtSplinePoint` _spline_road _returnvalue_2)))
    (`SplineMeshComponent.SetEndScale` _returnvalue (`KismetMathLibrary.MakeVector2D` _returnvalue_y_2 _returnvalue_z_2) true)
    (if (== _index 0)
      (`PrimitiveComponent.SetDefaultCustomPrimitiveDataFloat` _returnvalue 0 1.0)
      (elif (== _index (- (`SplineComponent.GetNumberOfSplinePoints` (`self.Spline_Road`)) 2))
        (`PrimitiveComponent.SetDefaultCustomPrimitiveDataFloat` _returnvalue 0 -1.0)))))