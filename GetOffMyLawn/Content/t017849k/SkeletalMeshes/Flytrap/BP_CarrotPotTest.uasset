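; Test actor for a carrot pot that glows, then animates the scale of a carrot mesh.
; BeginPlay applies a dynamic instance of the carrot pot VAT material to MushroomPotVATMesh and sets a ready flag.
; While the flag is set, Tick calls Play on a timeline driving EmissiveGlow.
; When it finishes, the pot switches to a default material and a second timeline drives CarrotLow's scale.
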(event `self.ReceiveBeginPlay`
  (bind _returnvalue (`PrimitiveComponent.CreateDynamicMaterialInstance` (`self.MushroomPotVAT_mesh`) 0 "/Game/t017849k/SkeletalMeshes/Flytrap/VATMI_CarrotPot.VATMI_CarrotPot" "VATMI"))
  (set `self.Instance` _returnvalue)
  (set `self.MaterialSet` true))

(event `self.ReceiveTick`
  (params (DeltaSeconds :type "Float (single-precision)"))
  (bind _mushroompotvat_mesh (`self.MushroomPotVAT_mesh`))
  (if (`self.MaterialSet`)
    (bind (_direction _alpha) (`Timeline|Timeline_0`)
      (:`Update`
        (`MeshComponent.SetScalarParameterValueOnMaterials` _mushroompotvat_mesh "EmissiveGlow" _alpha))
      (:`Finished`
        (`PrimitiveComponent.SetMaterial` _mushroompotvat_mesh 0 "/Game/t017849k/SkeletalMeshes/Carrot/default.default")
        (bind (_direction_2 _alpha_2) (`Timeline|Timeline_1`)
          (:`Update`
            (`SceneComponent.SetRelativeScale3D` (`self.Carrot_low`) (`KismetMathLibrary.Conv_DoubleToVector` _alpha_2))))))))

(fn `UserConstructionScript`)