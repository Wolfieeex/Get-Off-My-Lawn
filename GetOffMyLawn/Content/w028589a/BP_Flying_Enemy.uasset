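; Flying enemy Blueprint, a child class that attacks a tower when its DamageSphere begins an overlap.
; The overlap calls AttackTower without filtering the other actor, while the local Attack_Tower event is empty.
; GetHealth and GetSeedCount write fixed values into CharacterStats before returning them, so each call resets that stat.
; ModifyHealth and ModifySeedCount only forward to the parent, and a health debug string sits unconnected.
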(event `self.ReceiveBeginPlay`
  (`parent.ReceiveBeginPlay`))

(event `self.DamageSphere.OnComponentBeginOverlap`
  (params (OverlappedComponent :type "PrimitiveComponent Object Reference") (OtherActor :type "Actor Object Reference") (OtherComp :type "PrimitiveComponent Object Reference") (OtherBodyIndex :type Integer) (bFromSweep :type Boolean) (SweepResult :type "HitResult Structure (by ref)"))
  (`self.Attack_Tower`))

(event `Attack_Tower`)

(fn `GetHealth`
  (returns (Health :type "Float (double-precision)"))
  (bind _structout (setmembers `/Game/Characters/BS_CharacterStats` :`StructRef` (`self.CharacterStats`) :`Health` 100.0))
  (return (`.Health_9_0A2B731541A6848E04980BB2CB466D3B` (break `/Game/Characters/BS_CharacterStats` _structout))))

(fn `GetSeedCount`
  (returns (SeedCount :type Integer))
  (bind _structout (setmembers `/Game/Characters/BS_CharacterStats` :`StructRef` (`self.CharacterStats`) :`SeedCount` 1))
  (return (`.SeedCount_10_8B1B175242E26C8AD0EA33A9A109921F` (break `/Game/Characters/BS_CharacterStats` _structout))))

(fn `ModifyHealth`
  (params (Amount :type "Float (double-precision)") (`Positive?` :type Boolean))
  (locals (L_Health :type "Float (double-precision)"))
  (`parent.ModifyHealth` Amount `Positive?`))

(fn `ModifySeedCount`
  (params (Amount :type Integer) (`Positive?` :type Boolean))
  (`parent.ModifySeedCount` Amount `Positive?`))

(fn `UserConstructionScript`
  (`parent.UserConstructionScript`))