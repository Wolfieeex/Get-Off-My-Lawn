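; BP_Goal is the player's base, tracking its health and ending the game when that runs out.
; BeginPlay creates the goal HUD and starts a looping timer that polls health, showing the game-over widget and opening the main menu at zero.
; Interface damage events update the clamped health struct, refresh the HUD and trigger a one-shot under-attack handler for a temporary warning widget.
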(event `self.ReceiveBeginPlay`
  ;[0.8503 1 0.3375 1 50] Add to viewport
  (bind _returnvalue (`|CreateWidget` "/Game/d017162l/HUD/WBP_Goal_HUD.WBP_Goal_HUD_C"))
  (bind _output_get (set `self.BP_GoalRef` _returnvalue))
  (`UserWidget.AddToViewport` _output_get 0)
  (`/Game/d017162l/HUD/WBP_Goal_HUD.UpdateTextInfo` _output_get)
  (bind _returnvalue_2 (`KismetSystemLibrary.K2_SetTimerDelegate` (delegate `ChangeScene`) 0.356545 true))
  (set `self.NewVar_0` _returnvalue_2))

(event `/Game/Characters/BPI_Health.I_SubtractHealth`
  (params (Amount :type "Float (double-precision)"))
  ;[0.1964 1 0.1334] Lose health
  (`self.Update_Health` Amount)
  (set `self.CurrentHealth` Amount)
  ;[1 0.3959 0.3061 1 26] Call base under attack function
  (`/Game/d017162l/HUD/WBP_Goal_HUD.UpdateTextInfo` (`self.BP_GoalRef`))
  (`/Engine/EditorBlueprintResources/StandardMacros.DoOnce` false
    (:`Completed`
      (`self.Base is under attack`))))

(event `ChangeScene`
  ;[0.2333 0.3191 1 1 34] Game over screen
  (bind _health (`self.Get health`))
  (if (<= _health 0.0)
    (`KismetSystemLibrary.Delay` 1.0)
    (bind _returnvalue (`|CreateWidget` "/Game/d017162l/HUD/WBP_Game_Over.WBP_Game_Over_C"))
    (`UserWidget.AddToViewport` _returnvalue 0)
    (`KismetSystemLibrary.Delay` 1.5)
    (`GameplayStatics.OpenLevelBySoftObjectPtr` "/Game/Maps/MainMenu.MainMenu")
    (`KismetSystemLibrary.K2_ClearAndInvalidateTimerHandle` (`self.NewVar_0`))))

(event `Base is under attack`
  ;[0.6641 1 0.9601 1 42] Base under attack text pop-up
  (for _ (range 1)
    (`self.BP_GoalRef`
      (:`then`
        (if (`self.TowerUnderAttack`)
          (set `self.TowerUnderAttack` true)
          (if (`Widget.IsInViewport` (`self.BP_GoalRef`))
            (bind _returnvalue (`|CreateWidget` "/Game/d017162l/HUD/Player/WBP_BaseUnderAttack.WBP_BaseUnderAttack_C"))
            (`UserWidget.AddToViewport` _returnvalue 0)
            (`KismetSystemLibrary.Delay` 4.0)
            (`Widget.RemoveFromParent` _returnvalue))))
      (:`else`))))

(event `/Game/Characters/BPI_Health.I_AddHealth`
  (params (Amount :type "Float (double-precision)"))
  (bind _output_get (set `self.CurrentHealth` (+ (`.Current_Health_5_61057DF74851D8316BAADDB1CCCD4E9D` (break `/Game/d017162l/Sructs/ST_Goal_Health` (`self.ProgressBar`))) Amount)))
  (set `self.CurrentHealth` (`KismetMathLibrary.FClamp` _output_get 0.0 (`self.MaxHealth`))))

(event `UpdateText`)

(fn `Get health`
  (returns (Health :type "Float (double-precision)"))
  (return (`.Current_Health_5_61057DF74851D8316BAADDB1CCCD4E9D` (break `/Game/d017162l/Sructs/ST_Goal_Health` (`self.ProgressBar`)))))

(fn `PlayCameraShake`
  (`MatineeCameraShake.StartMatineeCameraShake` (`GameplayStatics.GetPlayerCameraManager` 0) "/Game/d017162l/Blueprints/BP_GoalCameraShake.BP_GoalCameraShake_C"))

(fn `Update_Health`
  (params (`Amount ` :type "Float (double-precision)"))
  (locals (L_Current_Health :type "Float (double-precision)"))
  (set `local.L_Current_Health` (- (`.Current_Health_5_61057DF74851D8316BAADDB1CCCD4E9D` (break `/Game/d017162l/Sructs/ST_Goal_Health` (`self.ProgressBar`))) `Amount `))
  (bind _output_get (set `local.L_Current_Health` (`KismetMathLibrary.FClamp` (`local.L_Current_Health`) 0.0 (`.Max_Health_4_81DC08F84AC8657A52C57192E268A698` (break `/Game/d017162l/Sructs/ST_Goal_Health` (`self.ProgressBar`))))))
  (setmembers `/Game/d017162l/Sructs/ST_Goal_Health` :`StructRef` (`self.ProgressBar`) :`Current_Health` _output_get)
  (if (<= _output_get 0.0)
    (`KismetSystemLibrary.PrintString` "GAME OVER")
    (`KismetSystemLibrary.K2_ClearAndInvalidateTimerHandle` (`self.Attack Handle`))))

(fn `UserConstructionScript`)