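; AI controller for MasterEnemy pawns that drives waypoint and player-sight behavior through the BT_MasterEnemy behavior tree.
; After a short delay on BeginPlay, it runs the tree and seeds the blackboard with the first waypoint as target.
; Sight perception sets or clears TargetPlayer for the player character and records LastKnownLocation when sight is lost.
; Tower-targeting logic is present but disconnected, so it never runs.
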(event `self.AIPerception.OnPerceptionUpdated`
  (params (UpdatedActors :type "Array of Actor Object Reference (by ref)")))

(event `self.AIPerception.OnTargetPerceptionUpdated`
  (params (Actor :type "Actor Object Reference") (Stimulus :type "AIStimulus Structure"))
  (`self.HandleSightSense` Actor Stimulus))

(event `self.ReceiveBeginPlay`
  (bind _returnvalue (`AIBlueprintHelperLibrary.GetBlackboard` null))
  (`KismetSystemLibrary.Delay` 1.0)
  (bind _asmaster_enemy (cast `/Game/w028589a/MasterEnemy` (`self.K2_GetPawn`)))
  (`self.RunBehaviorTree` "/Game/w028589a/BT_MasterEnemy.BT_MasterEnemy")
  (`BlackboardComponent.SetValueAsInt` _returnvalue (`self.CurrentWaypointKey`) 0)
  (`BlackboardComponent.SetValueAsObject` _returnvalue (`self.TargetActorKey`) (`|GetArrayItem` (`/Game/w028589a/MasterEnemy.Waypoints` _asmaster_enemy))))

(fn `HandleSightSense`
  (params (Actor :type "Actor Object Reference") (Stimulus :type "AIStimulus Structure"))
  (returns (NewParam :type "AIStimulus Structure"))
  (bind (_age _expirationage _strength _stimuluslocation _receiverlocation _tag _bsuccessfullysensed) (break `AIStimulus` (`local.Stimulus`)))
  (bind _returnvalue (`AIPerceptionSystem.GetSenseClassForStimulus` Stimulus))
  (if (== _returnvalue "/Script/AIModule.AISense_Sight")
    (if (== (`local.Actor`) (`GameplayStatics.GetPlayerCharacter` 0))
      (`BlackboardComponent.SetValueAsObject` (`self.Blackboard`) "TargetPlayer" (`KismetMathLibrary.SelectObject` (`GameplayStatics.GetPlayerCharacter` 0) null _bsuccessfullysensed))
      (if (not _bsuccessfullysensed)
        (`BlackboardComponent.SetValueAsVector` (`self.Blackboard`) "LastKnownLocation" _stimuluslocation))
      (else
        (return)))
    (else
      (return))))

(fn `UserConstructionScript`)