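; Player projectile, apparently for a plant tower, that steers toward MasterEnemy actors and damages them on contact.
; When an enemy enters the Guide volume, a sphere trace finds nearby objects and resets velocity toward each hit's predicted position using suggested toss velocity, so the last hit wins.
; Sphere overlap subtracts health from the enemy through an interface message and destroys the projectile.
; Tag-based nearest-target homing exists but is disconnected.
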(event `self.ReceiveBeginPlay`
  (set `self.ProjectileSpeed1` (`MovementComponent.GetMaxSpeed` (`self.ProjectileMovement`))))

(event `FindTarget`)

(event `self.Guide.OnComponentBeginOverlap`
  (params (OverlappedComponent :type "PrimitiveComponent Object Reference") (OtherActor :type "Actor Object Reference") (OtherComp :type "PrimitiveComponent Object Reference") (OtherBodyIndex :type Integer) (bFromSweep :type Boolean) (SweepResult :type "HitResult Structure (by ref)"))
  (bind _returnvalue (`self.K2_GetActorLocation`))
  (cast `/Game/w028589a/MasterEnemy` OtherActor)
  (bind _outhits (`KismetSystemLibrary.SphereTraceMultiForObjects` _returnvalue _returnvalue 150.0 (`|MakeArray` "ObjectTypeQuery7" :!type "EObjectTypeQuery Enum")))
  (for _array_element _outhits
    (bind (_bblockinghit _binitialoverlap _time _distance _location _impactpoint _normal _impactnormal _physmat _hitactor) (`GameplayStatics.BreakHitResult` _array_element))
    (bind _tossvelocity (`GameplayStatics.BlueprintSuggestProjectileVelocity` (`self.K2_GetActorLocation`) (+ (`self.K2_GetActorLocation` _hitactor) (* (/ (`self.GetDistanceTo` _hitactor) (`self.ProjectileSpeed1`)) (`self.GetVelocity` _hitactor))) (`self.ProjectileSpeed1`) 0.0 "DoNotTrace"))
    (set `MovementComponent.Velocity` _tossvelocity (`self.ProjectileMovement`))))

(event `self.Sphere.OnComponentBeginOverlap`
  (params (OverlappedComponent :type "PrimitiveComponent Object Reference") (OtherActor :type "Actor Object Reference") (OtherComp :type "PrimitiveComponent Object Reference") (OtherBodyIndex :type Integer) (bFromSweep :type Boolean) (SweepResult :type "HitResult Structure (by ref)"))
  (bind _asmaster_enemy (cast `/Game/w028589a/MasterEnemy` OtherActor))
  (message `/Game/Characters/BPI_Health.I_SubtractHealth` _asmaster_enemy 10.0)
  (`self.K2_DestroyActor`))

(fn `FindHomingTarget`
  (returns (HomingTarget :type "SceneComponent Object Reference"))
  (bind _outactors (`GameplayStatics.GetAllActorsOfClassWithTag` "/Script/Engine.Actor" "Homing"))
  (for _array_element _outactors
    (bind _returnvalue (`KismetMathLibrary.VSize` (- (`self.K2_GetActorLocation` _array_element) (`self.K2_GetActorLocation`))))
    (if (< _returnvalue (`self.Closest Distance`))
      (set `self.Closest Distance` _returnvalue)
      (set `self.HomingTarget` _array_element)))
  (return (`self.GetComponentByClass` (`self.HomingTarget`) "/Script/Engine.SceneComponent")))

(fn `UserConstructionScript`)