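; Homing projectile, filed under the plant tower assets, that seeks a target and damages enemies on contact.
; On BeginPlay it picks the closest actor tagged "Homing" within the initial ClosestDistance and feeds that actor's scene component to ProjectileMovement as the homing target.
; The target is chosen only once.
; Overlapping a MasterEnemy with its sphere sends a fixed subtract-health message, then destroys the projectile.
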(event `self.ReceiveBeginPlay`
  (`self.FindTarget`))

(event `FindTarget`
  (bind _projectilemovement (`self.ProjectileMovement`))
  (bind _homingtarget (`self.FindHomingTarget`))
  (set `ProjectileMovementComponent.HomingTargetComponent` _homingtarget _projectilemovement)
  (set `ProjectileMovementComponent.bIsHomingProjectile` true _projectilemovement))

(event `self.Sphere.OnComponentBeginOverlap`
  (params (OverlappedComponent :type "PrimitiveComponent Object Reference") (OtherActor :type "Actor Object Reference") (OtherComp :type "PrimitiveComponent Object Reference") (OtherBodyIndex :type Integer) (bFromSweep :type Boolean) (SweepResult :type "HitResult Structure (by ref)"))
  (bind _asmaster_enemy (cast `/Game/w028589a/MasterEnemy` OtherActor))
  (message `/Game/Characters/BPI_Health.I_SubtractHealth` _asmaster_enemy 10.0)
  (`self.K2_DestroyActor`))

(fn `FindHomingTarget`
  (returns (HomingTarget :type "SceneComponent Object Reference"))
  (bind _outactors (`GameplayStatics.GetAllActorsOfClassWithTag` "/Script/Engine.Actor" "Homing"))
  (for _array_element _outactors
    (bind _returnvalue (`KismetMathLibrary.VSize` (- (`self.K2_GetActorLocation` _array_element) (`self.K2_GetActorLocation`))))
    (if (< _returnvalue (`self.Closest Distance`))
      (set `self.Closest Distance` _returnvalue)
      (set `self.HomingTarget` _array_element)))
  (return (`self.GetComponentByClass` (`self.HomingTarget`) "/Script/Engine.SceneComponent")))

(fn `UserConstructionScript`)