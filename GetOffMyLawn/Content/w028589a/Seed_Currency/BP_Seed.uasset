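; BP_Seed is a seed currency pickup that increases the player's seed count when collected.
; A timeline animates its idle position and rotation from BeginPlay, stopping when anything overlaps the capsule.
; For a ThirdPersonCharacter, it adds SeedAmount, spawns an overlap Niagara effect and plays a pickup timeline toward a separate offset and rotation.
; A one-second Delay fired from that timeline's update then spawns the collect effect and destroys the actor.
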(event `self.ReceiveBeginPlay`
  (bind _startlocation (`self.StartLocation`))
  ;[1 1 1] Seed Movement
  (set `self.StartLocation` (`self.K2_GetActorLocation`))
  (set `self.StartRotation` (`self.K2_GetActorRotation`))
  (bind (_direction _alpha) (`Timeline|SeedMovement` :!label _label)
    (:`Update`
      (`self.K2_SetActorLocation` (`KismetMathLibrary.VLerp` _startlocation (+ _startlocation (`self.EndLocationOffset`)) _alpha))
      (`self.K2_SetActorRotation` (`KismetMathLibrary.RLerp` (`self.StartRotation`) (`self.EndRotation`) _alpha)))))

(event `self.Capsule.OnComponentBeginOverlap`
  (params (OverlappedComponent :type "PrimitiveComponent Object Reference") (OtherActor :type "Actor Object Reference") (OtherComp :type "PrimitiveComponent Object Reference") (OtherBodyIndex :type Integer) (bFromSweep :type Boolean) (SweepResult :type "HitResult Structure (by ref)"))
  (bind _startlocation (`self.StartLocation`))
  (`|ExecutionSequence`
    (:`then_0`
      (goto _label :!via `Stop`))
    (:`then_1`
      ;[1 1 1] Seed adding to UI
      (bind _asthird_person_character (cast `/Game/Blueprints/GameCore/ThirdPersonCharacter` OtherActor))
      (`/Game/Blueprints/GameCore/ThirdPersonCharacter.ModifySeedCount` _asthird_person_character (`self.SeedAmount`) true)
      ;[1 1 1] Seed Pick Up Movement
      (set `self.StartLocation` (`self.K2_GetActorLocation`))
      (set `self.StartRotation` (`self.K2_GetActorRotation`))
      (`NiagaraFunctionLibrary.SpawnSystemAtLocation` "/Game/w028589a/Seed_Currency/NS_SeedOverlap.NS_SeedOverlap" (`SceneComponent.K2_GetComponentLocation` (`self.SeedMesh`)))
      (bind (_direction _alpha) (`Timeline|PickupTimeline`)
        (:`Update`
          (`self.K2_SetActorLocation` (`KismetMathLibrary.VLerp` _startlocation (+ _startlocation (`self.EndLocationPickupOffset`)) _alpha))
          (`self.K2_SetActorRotation` (`KismetMathLibrary.RLerp` (`self.StartRotation`) (`self.EndRotationPickUp`) _alpha))
          (`KismetSystemLibrary.Delay` 1.0)
          (`NiagaraFunctionLibrary.SpawnSystemAtLocation` "/Game/w028589a/Seed_Currency/NS_SeedCollect.NS_SeedCollect" (+ (`SceneComponent.K2_GetComponentLocation` (`self.SeedMesh`)) (0.0 0.0 125.0)))
          (`self.K2_DestroyActor`))))))

(fn `UserConstructionScript`)